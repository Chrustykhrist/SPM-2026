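; Player character Blueprint that drives its own camera rig, with height handled separately from horizontal position.
; BeginPlay gives the SpringArm an absolute location at the actor's position plus a Z offset.
; Each Tick, CameraLag matches actor XY and passes height through FInterpTo, though no interp speed is set.
; Tick then pins the Camera to the capsule's XY, keeping the camera's own Z.
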(event EventBeginPlay
  (bind _returnvalue (Transformation|GetActorLocation))
  (bind _springarm (Variables|Default|GetSpringArm))
  (bind (_x _y _z) (Math|Vector|BreakVector _returnvalue))
  (Transformation|SetAbsolute _springarm true false false)
  (Transformation|SetWorldLocation _springarm (Math|Vector|MakeVector _x _y (+ _z (Variables|Default|GetSpringArmZOffset))) false false))

(event Collision|EventActorBeginOverlap
  (params (OtherActor :type Actor%20Object%20Reference)))

(event EventTick
  (params (DeltaSeconds :type Float%20%28single-precision%29))
  (bind _camera (Variables|Default|GetCamera))
  (bind _capsulecomponent (Variables|Default|GetCapsuleComponent))
  (bind _returnvalue (Transformation|GetWorldLocation _capsulecomponent))
  (bind (_x _y) (Math|Vector|BreakVector _returnvalue))
  (CallFunction|CameraLag)
  (Transformation|SetWorldLocation _camera (Math|Vector|MakeVector _x _y (.Z (Math|Vector|BreakVector (Transformation|GetWorldLocation _camera)))) false false))

(fn ConstructionScript)

(fn CameraLag
  (bind _returnvalue (Transformation|GetActorLocation))
  (bind _springarm (Variables|Default|GetSpringArm))
  (bind (_x _y _z) (Math|Vector|BreakVector _returnvalue))
  (Transformation|SetWorldLocation _springarm (Math|Vector|MakeVector _x _y (Math|Interpolation|FInterpTo (.Z (Math|Vector|BreakVector (Transformation|GetWorldLocation _springarm))) (+ _z (Variables|Default|GetSpringArmZOffset)) (Utilities|Time|GetWorldDeltaSeconds) 0.0)) false false))